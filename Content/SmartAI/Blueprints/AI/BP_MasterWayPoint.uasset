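; BP_MasterWayPoint is a waypoint actor for the SmartAI system that carries a position and a facing target.
; Its construction script caches WayPointFaceDirection as a world point projected along the actor's forward vector from slightly above its origin.
; It also sets Arrow visibility and Box in-game hiding from HideRotationArrow and ShowInGame, both acting opposite to their names because they are passed without negation.
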(fn `UserConstructionScript`
  (set `self.Way Point Face Direction` (+ (+ (`self.K2_GetActorLocation`) (0.0 0.0 80.0)) (* (`KismetMathLibrary.Conv_RotatorToVector` (`self.K2_GetActorRotation`)) 400.0)))
  (`SceneComponent.SetVisibility` (`self.Arrow`) (`self.Hide Rotation Arrow`) false)
  (`SceneComponent.SetHiddenInGame` (`self.Box`) (`self.Show In Game`) true))