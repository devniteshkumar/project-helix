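; AI controller for NPC enemies that runs BT_NPC and switches its blackboard state when the player is sensed.
; On possess, after a zero-length delay, it starts the tree, stores the player as AttackTarget and sets the initial state.
; Perception updates use CanSenseActor to check the player's stimuli by sense class; successful sight, hearing or damage all set the same second state.
; Nothing here reverts that state, and HandleSensed is empty.
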(event `self.ReceivePossess`
  (params (PossessedPawn :type "Pawn Object Reference"))
  (`KismetSystemLibrary.Delay` 0.0)
  (`self.RunBehaviorTree` "/Game/Enemy/Blueprints/AI/BT_NPC.BT_NPC")
  (`BlackboardComponent.SetValueAsObject` (`self.Blackboard`) "AttackTarget" (`GameplayStatics.GetPlayerCharacter` 0))
  (`BlackboardComponent.SetValueAsEnum` (`self.Blackboard`) (`self.StateKeyName`) (enumliteral `/Game/Enemy/Blueprints/AI/E_States` "NewEnumerator0")))

(event `self.AIPerception.OnPerceptionUpdated`
  (params (UpdatedActors :type "Array of Actor Object Reference (by ref)"))
  (for _array_element UpdatedActors
    (if (== _array_element (`GameplayStatics.GetPlayerCharacter` 0))
      (`|ExecutionSequence`
        (:`then_0`
          (bind _sensed (`self.CanSenseActor` _array_element "NewEnumerator0"))
          (if _sensed
            (`BlackboardComponent.SetValueAsEnum` (`self.Blackboard`) (`self.StateKeyName`) (enumliteral `/Game/Enemy/Blueprints/AI/E_States` "NewEnumerator1") :!label _label)))
        (:`then_1`
          (bind _sensed_2 (`self.CanSenseActor` _array_element "NewEnumerator1"))
          (if _sensed_2
            (goto _label)))
        (:`then_2`
          (bind _sensed_3 (`self.CanSenseActor` _array_element "NewEnumerator2"))
          (if _sensed_3
            (goto _label)))))))

(fn `CanSenseActor`
  (params (Actor :type "Actor Object Reference") (Senses :type "/Game/Enemy/Blueprints/AI/E_Senses Enum" :default "NewEnumerator3"))
  (returns (Sensed :type Boolean) (Stimulus :type "AIStimulus Structure"))
  (bind _info (`AIPerceptionComponent.GetActorsPerception` (`self.AIPerception`) Actor))
  (for _array_element (`.LastSensedStimuli` (break `ActorPerceptionBlueprintInfo` _info))
    (bind _returnvalue (`AIPerceptionSystem.GetSenseClassForStimulus` _array_element))
    (if (== _returnvalue (select `/Game/Enemy/Blueprints/AI/E_Senses` Senses :`NewEnumerator0` "/Script/AIModule.AISense_Sight" :`NewEnumerator1` "/Script/AIModule.AISense_Hearing" :`NewEnumerator2` "/Script/AIModule.AISense_Damage" :!type "Object Class Reference"))
      (return (`.bSuccessfullySensed` (break `AIStimulus` _array_element)) _array_element))))

(fn `HandleSensed`
  (params (Actor :type "Actor Object Reference")))

(fn `UserConstructionScript`)