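; BP_Spawn is an enemy spawner actor that periodically creates AI pawns at its own location.
; A looping 15-second timer started on BeginPlay spawns the configured PawnClass with its BehaviorTree.
; If the pawn is a BP_Melee, it receives the spawner's PatrolRoute, followed by a delay that leads nowhere.
; The Box overlap event is empty, and the logic to destroy the spawner for the player is disconnected.
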(event `self.ReceiveBeginPlay`
  (`KismetSystemLibrary.K2_SetTimerDelegate` (delegate `Spawn`) 15.0 true))

(event `Spawn`
  (bind _returnvalue (`AIBlueprintHelperLibrary.SpawnAIFromClass` (`self.Pawn Class`) (`self.Behavior Tree`) (`SceneComponent.K2_GetComponentLocation` (`self.DefaultSceneRoot`)) (struct) false null))
  (bind _asbp_melee (cast `/Game/Enemy/Blueprints/BP_Melee` _returnvalue))
  (set `/Game/Enemy/Blueprints/BP_Melee.PatrolRoute` (`self.Patrol Route`) _asbp_melee)
  (`KismetSystemLibrary.Delay` 5.0))

(event `self.Box.OnComponentBeginOverlap`
  (params (OverlappedComponent :type "PrimitiveComponent Object Reference") (OtherActor :type "Actor Object Reference") (OtherComp :type "PrimitiveComponent Object Reference") (OtherBodyIndex :type Integer) (bFromSweep :type Boolean) (SweepResult :type "HitResult Structure (by ref)")))

(fn `UserConstructionScript`)