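; BP_NPC is a melee enemy that takes bullet damage, swings a sword and dies with a montage.
; Bullet hits lower health, briefly show the health bar widget and report a damage event with the player as instigator; death disables collision, then destroys the actor.
; Attack plays a montage and signals its end, while the sword damages the player on overlap end.
; GetMovementSpeed switches walk and chase speeds; GetPatrolRoute is empty.
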(event `self.ReceiveBeginPlay`
  (bind _aswb_npc_health (cast `/Game/Enemy/Blueprints/WB_NPC_Health` (`WidgetComponent.GetUserWidgetObject` (`self.HealthBar`))))
  (bind _output_get (set `self.HealthBarRef` _aswb_npc_health))
  (set `/Game/Enemy/Blueprints/WB_NPC_Health.Health` (`self.Health`) _output_get))

(event `self.CapsuleComponent.OnComponentHit`
  (params (HitComponent :type "PrimitiveComponent Object Reference") (OtherActor :type "Actor Object Reference") (OtherComp :type "PrimitiveComponent Object Reference") (NormalImpulse :type "Vector Structure") (Hit :type "HitResult Structure (by ref)"))
  (bind _returnvalue (`GameplayStatics.GetPlayerCharacter` 0))
  (cast `/Game/FirstPerson/Blueprints/BP_Bullet` OtherActor)
  (`SceneComponent.SetVisibility` (`self.HealthBar`) true false)
  (bind _output_get (set `self.Health` (- (`self.Health`) 20.0)))
  (set `/Game/Enemy/Blueprints/WB_NPC_Health.Health` _output_get (`self.HealthBarRef`))
  (`AISense_Damage.ReportDamageEvent` self _returnvalue 0.0 (`self.K2_GetActorLocation` _returnvalue))
  (if (<= (`self.Health`) 0.0)
    (`self.StopAnimMontage` self "/Game/Enemy/Blueprints/AM_Attack.AM_Attack")
    (set `CharacterMovementComponent.MaxWalkSpeed` 0.0 (`self.CharacterMovement`))
    (`PrimitiveComponent.SetCollisionEnabled` (`self.CapsuleComponent`) "NoCollision")
    (`PrimitiveComponent.SetCollisionEnabled` (`self.Mesh`) "NoCollision")
    (`PrimitiveComponent.SetCollisionEnabled` (`self.Cylinder`) "NoCollision")
    (`PrimitiveComponent.SetCollisionEnabled` (`self.Sphere`) "NoCollision")
    (`PrimitiveComponent.SetCollisionEnabled` (`self.Sword`) "NoCollision")
    (`PrimitiveComponent.SetCollisionEnabled` (`self.HealthBar`) "NoCollision")
    (bind _returnvalue_2 (`self.PlayAnimMontage` "/Game/Mixamo/AM_Death.AM_Death"))
    (`KismetSystemLibrary.Delay` _returnvalue_2)
    (`self.K2_DestroyActor`)
    (else
      (`KismetSystemLibrary.Delay` 2.0)
      (`SceneComponent.SetVisibility` (`self.HealthBar`) false false))))

(event `Attack`
  (if (> (`self.Health`) 0.0)
    (`|PlayMontage` (`self.Mesh`) "/Game/Enemy/Blueprints/AM_Attack.AM_Attack" 1.0 0.0 "None" false
      (:`OnCompleted`
        _)
      (:`OnInterrupted`
        _))
    (`self.OnAttackEnd`)))

(event `self.Sword.OnComponentEndOverlap`
  (params (OverlappedComponent :type "PrimitiveComponent Object Reference") (OtherActor :type "Actor Object Reference") (OtherComp :type "PrimitiveComponent Object Reference") (OtherBodyIndex :type Integer))
  (bind _asbp_first_person_character (cast `/Game/FirstPerson/Blueprints/BP_FirstPersonCharacter` OtherActor))
  (`/Game/FirstPerson/Blueprints/BP_FirstPersonCharacter.TakeDamage` _asbp_first_person_character))

(fn `GetMovementSpeed`
  (params (Speeds :type "/Game/Enemy/Blueprints/Enum_Speed Enum" :default "NewEnumerator0"))
  (returns (SpeedValue :type "Float (double-precision)"))
  (set `CharacterMovementComponent.MaxWalkSpeed` (select `/Game/Enemy/Blueprints/Enum_Speed` Speeds :`NewEnumerator0` 300.0 :`NewEnumerator1` 500.0 :!type "Float (single-precision)") (`self.CharacterMovement`))
  (return 0.0))

(fn `GetPatrolRoute`
  (returns (PatrolRoute :type "/Game/Enemy/Blueprints/BP_PatrolRoute Object Reference"))
  (return null))

(fn `UserConstructionScript`)